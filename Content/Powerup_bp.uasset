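; Powerup pickup Blueprint that grants a random special ability to an overlapping MrCharacterPlayer that has none.
; On overlap it casts the actor to the player class and proceeds only if GetAbility returns -1.
; A weighted roll over the thief, collapse and swallow chances picks the ability, sets the matching player mesh and special ability, then destroys the pickup.
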(event Collision|EventActorBeginOverlap
  (params (OtherActor :type Actor%20Object%20Reference))
  (bind _asmr_character_player (Utilities|Casting|CastToMrCharacterPlayer OtherActor)
    (:then
      (bind _output_get (Variables|Default|SetPlayer _asmr_character_player))
      (bind _returnvalue (Class|MrCharacter|GetAbility _output_get))
      (if (== _returnvalue -1)
        (bind _output_get_2 (Variables|Default|SetrandVal (Math|Random|RandomFloatinRange 0.0 (+ (+ (Variables|Default|GetThiefChance) (Variables|Default|GetCollapseChance)) (Variables|Default|GetSwallowChance)))))
        (if (<= _output_get_2 (Variables|Default|GetThiefChance))
          (Default|SetPlayerMesh (Variables|Default|GetPlayer) "/Game/Animations/MrThief.MrThief")
          (Class|MrCharacter|SetSpecialAbility (Variables|Default|GetPlayer) (Variables|Default|GetPA_THIEF))
          (Actor|DestroyActor :!label _label)
          (elif (<= (- _output_get_2 (Variables|Default|GetThiefChance)) (Variables|Default|GetCollapseChance))
            (Default|SetPlayerMesh (Variables|Default|GetPlayer) "/Game/Animations/MrCollapse.MrCollapse")
            (Class|MrCharacter|SetSpecialAbility (Variables|Default|GetPlayer) (Variables|Default|GetPA_COLLAPSE))
            (goto _label)
            (elif (<= (- (- _output_get_2 (Variables|Default|GetThiefChance)) (Variables|Default|GetCollapseChance)) (Variables|Default|GetSwallowChance))
              (Default|SetPlayerMesh (Variables|Default|GetPlayer) "/Game/Animations/MrSwallow.MrSwallow")
              (Class|MrCharacter|SetSpecialAbility (Variables|Default|GetPlayer) (Variables|Default|GetPA_SWALLOW))
              (goto _label)
              (else
                (Development|PrintString "Somehow managed to not find a powerup!")))))))
    (:CastFailed
      (Development|PrintString "Not sure what we could have actually collided with..."))))

(fn ConstructionScript)