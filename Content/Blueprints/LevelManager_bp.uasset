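; Level manager that builds a Width by Height grid of LevelSegment_bp tiles when its CreateLevel event runs.
; The first segment spawns with a default transform, and later ones are spaced by the previous segment's DesertTileMesh local bounds plus padding.
; Each segment is stored in LevelPieces and passed to GetDistanceFromCenter.
; DoOneThing is a small add-a-constant function that the level build does not use.
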(event Custom|CreateLevel
  (for _index (range 0 (- (Variables|Default|Getwidth) 1))
    (for _index_2 (range 0 (- (Variables|Default|Getheight) 1))
      (if (Utilities|IsValid (Variables|Default|GetlastPlaced))
        (bind _returnvalue (Game|SpawnActorfromClass "/Game/Blueprints/LevelSegment_bp.LevelSegment_bp_C" (Math|Transform|MakeTransform (Math|Vector|MakeVector (* 2 (* _index (+ (.x (.Max (Components|StaticMesh|GetLocalBounds (Variables|/Game/Blueprints/LevelSegment_bp.LevelSegment_bp_C|GetDesertTile_Mesh (Variables|Default|GetlastPlaced))))) 5.0))) (* 2 (* _index_2 (+ (.y (.Max (Components|StaticMesh|GetLocalBounds (Variables|/Game/Blueprints/LevelSegment_bp.LevelSegment_bp_C|GetDesertTile_Mesh (Variables|Default|GetlastPlaced))))) 5.0))) 0.0) "0, 0, 0" "1,1,1") "Undefined" 0 0))
        (Variables|Default|SetlastPlaced _returnvalue)
        (else
          (bind _returnvalue_2 (Game|SpawnActorfromClass "/Game/Blueprints/LevelSegment_bp.LevelSegment_bp_C" (Math|Transform|MakeTransform (Math|Vector|MakeVector 0.0 0.0 0.0) "0, 0, 0" "1,1,1") "Undefined" 0 0))
          (Variables|Default|SetlastPlaced _returnvalue_2)))
      (Utilities|Array|Add (Variables|Default|GetlevelPieces) (Variables|Default|GetlastPlaced))
      (Class|LevelManager|GetDistancefromCenter (Variables|Default|GetlastPlaced)))))

(fn ConstructionScript)

(fn DoOneThing
  (params (NewParam :type Integer))
  (return (+ NewParam 5)))