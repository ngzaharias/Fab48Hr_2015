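; MrCharacterPlayer is the player character Blueprint, adding charge-attack hit handling and a swappable static mesh.
; Each ChargeTick checks the ChargeTrigger for other overlapping MrCharacterPlayer actors, pushes them along the controller's aim direction scaled by ChargeImpactForce, then calls ChargeFinish.
; SetPlayerMesh swaps the static mesh on the RenderMesh component.
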(event EventChargeTick
  (for _array_element (Collision|GetOverlappingActors (Variables|Default|GetChargeTrigger) "MrCharacterPlayer_C" :!class /Script/Engine.PrimitiveComponent)
    (bind _asmr_character_player (Utilities|Casting|CastToMrCharacterPlayer _array_element))
    (if (not (== _array_element self))
      (Physics|AddImpulse (Variables|/Script/Engine.Character|GetCharacterMovement _asmr_character_player) (* (Math|Rotator|GetRotationXVector (Pawn|GetControlRotation (Pawn|GetController) :!class /Script/Engine.Controller)) (Variables|Default|GetChargeImpactForce)) false)
      (Class|MrCharacter|ChargeFinish))))

(fn ConstructionScript)

(fn SetPlayerMesh
  (params (newMesh :type Static%20Mesh%20Object%20Reference))
  (Components|StaticMesh|SetStaticMesh (Variables|Default|GetRenderMesh) newMesh))